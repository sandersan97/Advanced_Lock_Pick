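; Player controller for the Advanced Lock Pick system that lets the player start a lock-pick interaction.
; Pressing Q calls StartInteractCL on its lock-pick interactor component, passing a line from the character's capsule along its forward vector.
; The call also supplies a hardcoded lock-pick transform, a pick count, a WorldDynamic object filter and persistent debug drawing.
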(event `Key|Q`
  (params (Key :type "Key Structure"))
  (bind _capsulecomponent (`Character.CapsuleComponent` (`GameplayStatics.GetPlayerCharacter` 0)))
  (bind _returnvalue (`SceneComponent.K2_GetComponentLocation` _capsulecomponent))
  ;[1 1 1] Spawn Interaction
  (:`Pressed`
    (`/Game/Advanced_Lock_Pick/Blueprints/Interactor_Lock_Pick_Component_BP.Start_Interact_CL` (`self.Interactor_Lock_Pick_Component_BP`) _returnvalue (+ _returnvalue (`KismetMathLibrary.MakeVector` (* (.x (`SceneComponent.GetForwardVector` _capsulecomponent)) 2000.0) (* (.y (`SceneComponent.GetForwardVector` _capsulecomponent)) 2000.0) (* (.z (`SceneComponent.GetForwardVector` _capsulecomponent)) 2000.0))) (`KismetMathLibrary.MakeTransform` (944.0 1744.0 0.0)) (`|MakeArray` "ObjectTypeQuery2" :!type "EObjectTypeQuery Enum") (`|MakeArray` self :!type "Actor Object Reference") "Persistent" 10)))

(fn `UserConstructionScript`)