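; Interactor component for the Advanced Lock Pick system that finds locked objects and opens their picking session.
; A server-side multi line trace finds an actor and component by lock-pick tags, checking that it is locked.
; The client then starts lock opening with the pick count, spawn transform and lock details.
; Lock-change events return through the server and multicast to set the lock status.
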(event `Start_Interact_CL`
  (params (Start_Location :type "Vector Structure") (End_Location :type "Vector Structure") (Lock_Pick_Transform :type "Transform Structure") (ObjectTypes :type "Array of EObjectTypeQuery Enum (by ref)") (ActorsToIgnore :type "Array of Actor Object Reference (by ref)") (DrawDebugType :type "EDrawDebugTrace Enum" :default "None") (Pick_Count :type Integer))
  ;[1 1 1] Start interaction and calculate if hited item is locked with LockPick System, if yes open Unlocking system if not do nothing,
  (`self.Start_Interact_SR` Start_Location End_Location Lock_Pick_Transform ObjectTypes ActorsToIgnore DrawDebugType Pick_Count))

(event `Start_Interact_SR`
  (params (Start :type "Vector Structure") (End :type "Vector Structure") (Lock_Pick_Transform :type "Transform Structure") (ObjectTypes :type "Array of EObjectTypeQuery Enum (by ref)") (ActorsToIgnore :type "Array of Actor Object Reference (by ref)") (DrawDebugType :type "EDrawDebugTrace Enum" :default "None") (Pick_Count :type Integer))
  ;[1 1 1] Start interaction and calculate if hited item is locked with LockPick System, if yes open Unlocking system if not do nothing,
  (bind _outhits (`KismetSystemLibrary.LineTraceMultiForObjects` Start End ObjectTypes false ActorsToIgnore DrawDebugType))
  (for _array_element _outhits
    (bind (_bblockinghit _binitialoverlap _time _distance _location _impactpoint _normal _impactnormal _physmat _hitactor) (`GameplayStatics.BreakHitResult` _array_element))
    (if (and _bblockinghit (`Actor.ActorHasTag` _hitactor "Lock_Pick_Actor"))
      (for _array_element_2 (`Actor.GetComponentsByTag` _hitactor "/Game/Advanced_Lock_Pick/Blueprints/Lock_Pick_Component_BP.Lock_Pick_Component_BP_C" "Lock_Pick_Component")
        (`/Engine/EditorBlueprintResources/StandardMacros.IsValid` _array_element_2
          (:`Is Valid`
            (if (`/Game/Advanced_Lock_Pick/Blueprints/Lock_Pick_Component_BP.Get_Lock_Status` _array_element_2)
              (`self.Open_Lock_CL` _array_element_2 Pick_Count Lock_Pick_Transform (`/Game/Advanced_Lock_Pick/Blueprints/Lock_Pick_Component_BP.Get_Lock_Details` _array_element_2))
              (break)))))
      (break))))

(event `Open_Lock_CL`
  (params (Target :type "/Game/Advanced_Lock_Pick/Blueprints/Lock_Pick_Component_BP Object Reference") (Picks_Count :type Integer) (Spawn_Transform :type "Transform Structure") (Locker_Details_Structure :type "/Game/Advanced_Lock_Pick/Blueprints/Other/Structures/Locker_Details_Structure Structure (by ref)"))
  ;[1 1 1] Start interaction and calculate if hited item is locked with LockPick System, if yes open Unlocking system if not do nothing,
  (add `self.On_Lock_Pick_Changed` (delegate `On_Lock_Changed`))
  (`/Game/Advanced_Lock_Pick/Blueprints/Lock_Pick_Component_BP.Start_Lock_Open` Target Picks_Count Spawn_Transform Locker_Details_Structure))

(event `On_Lock_Changed` :!signature `self.On_Lock_Pick_Changed`
  (params (Lock_Unlock :type Boolean))
  ;[1 1 1] Start interaction and calculate if hited item is locked with LockPick System, if yes open Unlocking system if not do nothing,
  (`self.Lock_Change_SR` (stale `Open_Lock_CL` Target) Lock_Unlock))

(event `Lock_Change_SR`
  (params (Target :type "/Game/Advanced_Lock_Pick/Blueprints/Lock_Pick_Component_BP Object Reference") (Status :type Boolean))
  ;[1 1 1] Start interaction and calculate if hited item is locked with LockPick System, if yes open Unlocking system if not do nothing,
  (`self.Lock_Change_Multy` Target Status))

(event `Lock_Change_Multy`
  (params (Target :type "/Game/Advanced_Lock_Pick/Blueprints/Lock_Pick_Component_BP Object Reference") (Status :type Boolean))
  ;[1 1 1] Start interaction and calculate if hited item is locked with LockPick System, if yes open Unlocking system if not do nothing,
  (`/Game/Advanced_Lock_Pick/Blueprints/Lock_Pick_Component_BP.Set_Lock_Status` Target Status))