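; Actor component that gives its owner a pickable lock, holding the lock's stick configuration and locked/unlocked state.
; On BeginPlay it tags itself and its owner to tell lock components and lock actors apart.
; Start_Lock_Open replaces any previous pick actor with a new Lock_Pick_Main_BP, configured from the passed locker details and pick count.
; Accessors expose the lock details and status, and setters update the status.
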(event `self.ReceiveBeginPlay`
  (bind _returnvalue (`self.GetOwner`))
  (bind _tags (`Actor.Tags` _returnvalue))
  ;[1 1 1] Add Lock Pick Tag on begin inside actor owners of this component and inside this component for understand which is what
  (`KismetArrayLibrary.Array_Add` (`self.ComponentTags`) "Lock_Pick_Component")
  (`/Engine/EditorBlueprintResources/StandardMacros.IsValid` _returnvalue
    (:`Is Valid`
      (if (not (`KismetArrayLibrary.Array_Contains` _tags "Lock_Pick_Actor"))
        (`KismetArrayLibrary.Array_Add` _tags "Lock_Pick_Actor")))))

(event `Start_Lock_Open`
  (params (Picks_Count :type Integer) (Spawn_Transform :type "Transform Structure") (Locker_Details_Structure :type "/Game/Advanced_Lock_Pick/Blueprints/Other/Structures/Locker_Details_Structure Structure (by ref)"))
  (bind (_block_sticks_number _random_sticks_number _sticks_enumeration _random_sticks_enumeration _locked_unlocked _sticks_enable_rand_percents) (break `/Game/Advanced_Lock_Pick/Blueprints/Other/Structures/Locker_Details_Structure` Locker_Details_Structure))
  (set `self.Picks_Count` Picks_Count)
  (bind _spawned_lock_pick (`self.Spawned_Lock_Pick`)
    (:`then`
      (`Actor.K2_DestroyActor` _spawned_lock_pick))
    (:`else`
      _))
  (bind _returnvalue (`|SpawnActorFromClass` "/Game/Advanced_Lock_Pick/Blueprints/Lock_Pick_Main_BP.Lock_Pick_Main_BP_C" Spawn_Transform "AdjustIfPossibleButAlwaysSpawn" "OverrideRootScale" null _block_sticks_number _random_sticks_number _sticks_enumeration _random_sticks_enumeration _locked_unlocked _sticks_enable_rand_percents (`self.Picks_Count`) null))
  (set `self.Spawned_Lock_Pick` _returnvalue))

(event `Set_Locker_Status_SR`
  (params (Status :type Boolean))
  (set `self.Locked_Unlocked` Status))

(fn `Get_Lock_Details`
  (returns (NewParam :type "/Game/Advanced_Lock_Pick/Blueprints/Other/Structures/Locker_Details_Structure Structure"))
  (return (make `/Game/Advanced_Lock_Pick/Blueprints/Other/Structures/Locker_Details_Structure` (`self.Block_Sticks_Number`) (`self.Random_Sticks_Number`) (`self.Sticks_Enumeration`) (`self.Random_Sticks_Enumeration`) (`self.Locked_Unlocked`) (`self.Sticks_Enable_Rand_Percents`))))

(fn `Get_Lock_Status`
  (returns (Result :type Boolean))
  (return (`self.Locked_Unlocked`)))

(fn `Set_Lock_Status`
  (params (Locked_Unlocked :type Boolean))
  (set `self.Locked_Unlocked` Locked_Unlocked))