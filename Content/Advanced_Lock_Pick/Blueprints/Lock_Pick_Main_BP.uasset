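; Lock-picking minigame actor that builds a lock of fixed or random pin count, isolates it for RenderCam and opens its widget.
; Pick move and press events start looping timers that step the pick between pins or down and up.
; Each press rolls a per-pin percentage chance, and failing the SticksEnumeration order check resets the pins.
; When all pins are set, it notifies the player controller's interactor component and reveals the widget's open button.
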(event `self.ReceiveBeginPlay`
  ;[1 1 1] On spawn start sections calculations and spawn its
  (`self.Start_Sections_Calculation`))

(event `Start_Sections_Calculation`
  (if (`self.Random_Sticks_Number`)
    (set `self.Selected_Rand_Number` (`self.Calculation_Rand_Sticks_Number`))
    (else
      (set `self.Selected_Rand_Number` (`self.Block_Sticks_Number`))))
  (for _index (range (`self.Selected_Rand_Number`))
    (bind _returnvalue (`|AddComponentByClass` "/Script/Engine.StaticMeshComponent" false (`SceneComponent.GetRelativeTransform` (`self.DefaultSceneRoot`))))
    (`SceneCaptureComponent.ShowOnlyComponent` (`self.Render_Cam`) _returnvalue)
    (bind _returnvalue_2 (`StaticMeshComponent.SetStaticMesh` _returnvalue "/Game/Advanced_Lock_Pick/Meshes/Static/ST_Lock_Middle_Wall.ST_Lock_Middle_Wall"))
    (if _returnvalue_2
      ;[1 1 1] Spawn and attach Movable Stick to it Section
      (bind _returnvalue_3 (`|AddComponentByClass` "/Script/Engine.SkeletalMeshComponent" true (`KismetMathLibrary.MakeTransform` (0.0 0.0 0.0))))
      (`SceneCaptureComponent.ShowOnlyComponent` (`self.Render_Cam`) _returnvalue_3)
      (bind _returnvalue_4 (`SceneComponent.K2_AttachToComponent` _returnvalue_3 _returnvalue "None" "SnapToTarget" "SnapToTarget" "SnapToTarget" true))
      (if _returnvalue_4
        (`SkinnedMeshComponent.SetSkinnedAssetAndUpdate` _returnvalue_3 "/Game/Advanced_Lock_Pick/Meshes/Skeletal/SkeletalMesh_Stick.SkeletalMesh_Stick" true)
        ;[1 1 1] Collect and sort all spawned sticks with its sections and set location for spawned section
        (`BlueprintMapLibrary.Map_Add` (`self.Spawned_Sections`) _returnvalue _returnvalue_3)
        (`SceneComponent.K2_SetRelativeTransform` _returnvalue (`KismetMathLibrary.MakeTransform` (`KismetMathLibrary.MakeVector` (+ 2.4416 (* 1.568 (- (* 2.0 (`BlueprintMapLibrary.Map_Length` (`self.Spawned_Sections`))) 1.0))) 0.0 2.9)) false true)
        ;[1 1 1] Set the Sections number and its Unlock status
        (`BlueprintMapLibrary.Map_Add` (`self.Sections_Status`) (+ _index 1)))))
  ;[1 1 1] Spawn andd set Location of last the End Section
  (bind _keys (`BlueprintMapLibrary.Map_Keys` (`self.Spawned_Sections`)))
  (bind _output (`|GetArrayItem` _keys (`KismetArrayLibrary.Array_LastIndex` _keys)))
  (`/Engine/EditorBlueprintResources/StandardMacros.IsValid` _output
    (:`Is Valid`
      (bind _returnvalue_5 (`|AddComponentByClass` "/Script/Engine.StaticMeshComponent" false (`KismetMathLibrary.MakeTransform` (`KismetMathLibrary.MakeVector` (+ (.x (`SceneComponent.RelativeLocation` _output)) 1.5)))))
      (`SceneCaptureComponent.ShowOnlyComponent` (`self.Render_Cam`) _returnvalue_5)
      (bind _returnvalue_6 (`StaticMeshComponent.SetStaticMesh` _returnvalue_5 "/Game/Advanced_Lock_Pick/Meshes/Static/ST_Lock_End_Wall.ST_Lock_End_Wall"))
      (if _returnvalue_6
        ;[1 1 1] Spawn Lock Pick Widget to see how this work and work with it
        (bind _returnvalue_7 (`|CreateWidget` "/Game/Advanced_Lock_Pick/Widgets/Lock_Pick_Widget_BP.Lock_Pick_Widget_BP_C" (`GameplayStatics.GetPlayerController` 0) self))
        (bind _output_get (set `self.Spawned_Locker_Widget` _returnvalue_7))
        (`UserWidget.AddToViewport` _output_get (`self.Zorder`))
        ;[1 1 1] Activate Inputs
        (`self.Activate Lock_Pick_Controll`)
        ;[1 1 1] Pick Controllers Binding and its functions
        (add `self.On_Pick_Moved_Right` (delegate `On Pick Move To Right Called`))
        (add `self.On_Pick_Moved_Left` (delegate `On Pick Move To Left Called`))
        (add `self.On_Pick_Activated` (delegate `On Pick Activate Called`))
        (add `self.On_Locker_Unlocked` (delegate `On_Locker_Unlocked_Event`))))))

(event `On Pick Move To Right Called`
  ;[1 1 1] Pick Controllers Binding and its functions
  (bind _returnvalue (`KismetSystemLibrary.K2_SetTimerDelegate` (delegate `Moving To Right`) 0.025 true))
  (set `self.Moving to Right Timer` _returnvalue))

(event `On_Locker_Unlocked_Event`
  ;[1 1 1] Pick Controllers Binding and its functions
  (`self.Locker Unlock Status Change`))

(event `On Pick Move To Left Called`
  ;[1 1 1] Pick Controllers Binding and its functions
  (bind _returnvalue (`KismetSystemLibrary.K2_SetTimerDelegate` (delegate `Move To Left`) 0.025 true))
  (set `self.Moving to Left Timer` _returnvalue))

(event `On Pick Activate Called`
  ;[1 1 1] Pick Controllers Binding and its functions
  (bind _returnvalue (`KismetSystemLibrary.K2_SetTimerDelegate` (delegate `Move Down`) 0.025 true))
  (set `self.Moving Down Timer` _returnvalue))

(event `Moving To Right`
  ;[1 1 1] Pick Controllers Binding and its functions
  (`self.Move_Pick_Right` (`self.Moving to Right Timer`)))

(event `Move To Left`
  ;[1 1 1] Pick Controllers Binding and its functions
  (`self.Move_Pick_Left` (`self.Moving to Left Timer`)))

(event `Move Down`
  ;[1 1 1] Pick Controllers Binding and its functions
  (`self.Down_Pick_Pisition` (`self.Moving Down Timer`)))

(event `Locker Unlock Status Change`
  (bind _returnvalue (`GameplayStatics.GetPlayerController` 0))
  (bind _returnvalue_2 (`self.GetComponentsByTag` _returnvalue "/Game/Advanced_Lock_Pick/Blueprints/Interactor_Lock_Pick_Component_BP.Interactor_Lock_Pick_Component_BP_C" "Lock_Pick_Interactor"))
  (bind _output (`|GetArrayItem` _returnvalue_2))
  ;[1 1 1] Logic which activate it self  if Door Opened or closed and change this status on server and for all players.
  (`|ExecutionSequence`
    (:`then_0`
      (`/Engine/EditorBlueprintResources/StandardMacros.IsValid` _returnvalue
        (:`Is Valid`
          (if (`KismetArrayLibrary.Array_IsValidIndex` _returnvalue_2)
            (`/Engine/EditorBlueprintResources/StandardMacros.IsValid` _output
              (:`Is Valid`
                (`/Game/Advanced_Lock_Pick/Blueprints/Interactor_Lock_Pick_Component_BP.On_Lock_Pick_Changed` _output false)
                ;[0.3802 0.1219 0] Demo
                (`KismetSystemLibrary.PrintString` "Yeeess! Locker Unlocked Succesful" true true (struct :`R` 0.021804 :`G` 1.0 :`A` 1.0) 15.0)))))))
    (:`then_1`
      ;;[1 1 1] Close and return button from Widget set to visible on all sticks activated succesful
      (bind _spawned_locker_widget (`self.Spawned_Locker_Widget`)
        (:`then`
          (set `/Game/Advanced_Lock_Pick/Widgets/Lock_Pick_Widget_BP.Open_Button_Visibillity` "Visible" _spawned_locker_widget))
        (:`else`)))))

(fn `Activate Lock_Pick_Controll`
  (`EnhancedInputSubsystemInterface.AddMappingContext` (pcsubsystem `EnhancedInputLocalPlayerSubsystem` (`GameplayStatics.GetPlayerController` 0)) "/Game/Advanced_Lock_Pick/Inputs/Advanced_Lock_Pick_Input_Mapping.Advanced_Lock_Pick_Input_Mapping" 0 (make `ModifyContextOptions` true true))
  (`WidgetBlueprintLibrary.SetInputMode_UIOnlyEx` (`GameplayStatics.GetPlayerController` 0) (`self.Spawned_Locker_Widget`)))

(fn `Add Pick_Position`
  (returns (`Is_Succes?` :type Boolean))
  (if (`self.Is Pick In Up Location`)
    (bind _keys (`BlueprintMapLibrary.Map_Keys` (`self.Spawned_Sections`)))
    (bind _returnvalue (`KismetArrayLibrary.Array_Length` _keys))
    (if (< (`self.Pick_Position`) _returnvalue)
      (set `self.Pick_Position` (`KismetMathLibrary.Clamp` (+ (`self.Pick_Position`) 1) 1 _returnvalue))
      (set `self.Do_Once_Right` false)
      (`self.Refresh Timers`)
      (`self.On_Pick_Moved_Right`)
      (return true)
      (else
        (return false)))
    (else
      (return false))))

(fn `Calculation_Rand_Sticks_Enumeration`
  (returns (Result :type "Array of Integer"))
  (locals (Selected_Numbers :type "Array of Integer") (Random_Stick_Number :type Integer :default 5))
  (bind _selected_numbers (`local.Selected_Numbers`))
  (bind _random_stick_number (`local.Random_Stick_Number`))
  (bind _returnvalue (`KismetMathLibrary.RandomIntegerInRange` 0 _random_stick_number))
  (if (`self.Random_Sticks_Number`)
    (set `local.Random_Stick_Number` (`self.Calculation_Rand_Sticks_Number`)))
  (while (and (`KismetArrayLibrary.Array_Contains` _selected_numbers _returnvalue) (< (`KismetArrayLibrary.Array_Length` _selected_numbers) _random_stick_number))
    (`KismetArrayLibrary.Array_Add` (`local.Selected_Numbers`) _returnvalue))
  (return (`local.Selected_Numbers`)))

(fn `Calculation_Rand_Sticks_Number`
  (returns (Result :type Integer))
  (return (`KismetMathLibrary.RandomIntegerInRange` 1 6)))

(fn `Down_Pick_Pisition`
  (params (`Timer Handle` :type "TimerHandle Structure"))
  (locals (Unlock_Status_Local :type Boolean))
  (bind (_random_result _end_location) (`self.Get Pick Down Location`))
  (bind _returnvalue (- (`self.Pick_Position`) 1))
  (bind _z (.z (`SceneComponent.RelativeLocation` (`self.Pick`))))
  (bind _returnvalue_2 (`KismetMathLibrary.MakeVector` (.x (`SceneComponent.RelativeLocation` (`self.Pick`))) (.y (`SceneComponent.RelativeLocation` (`self.Pick`))) 15.65))
  (if (and (not (`KismetSystemLibrary.K2_IsTimerActiveHandle` (`self.Moving to Right Timer`))) (not (`KismetSystemLibrary.K2_IsTimerActiveHandle` (`self.Moving to Left Timer`))))
    (if (`self.Do_Once_Down`)
      ;[1 1 1] Calculate is pick location on end location if not continue to change but if yes stop moving timer and reset do once.
      (if (and (== (`SceneComponent.RelativeLocation` (`self.Pick`)) (`self.End_Pick_Location`) :`ErrorTolerance` 0.1) (`self.Up_Down_Direction`))
        (if (`KismetSystemLibrary.K2_IsTimerActiveHandle` (`local.Timer Handle`))
          (`KismetSystemLibrary.K2_ClearAndInvalidateTimerHandle` (`local.Timer Handle`))
          (set `self.Do_Once_Down` false)
          (set `self.Up_Down_Direction` false)
          ;[1 0 0] Here set all sticks to return to default like unlocked and remove this timer
          (if (not (`self.Stick Activation Conditions`))
            (`self.Return_All_Sticks_Def`)))
        (else
          ;[1 1 1] On end to move pick down reverce it to move Up and change it movement direction status
          (if (== (`SceneComponent.RelativeLocation` (`self.Pick`)) (`self.End_Pick_Location`) :`ErrorTolerance` 0.1)
            (bind _output_get (set `self.Start_Pick_Location` (`self.End_Pick_Location`)))
            (set `self.End_Pick_Location` (`KismetMathLibrary.MakeVector` (.x _output_get) (.y _output_get) 15.65))
            (set `self.Up_Down_Direction` true)
            (else
              ;[1 1 1] Calculate how much need to move to right the Pick location and change it Down
              (`SceneComponent.K2_SetRelativeLocation` (`self.Pick`) (`KismetMathLibrary.MakeVector` (.x (`SceneComponent.RelativeLocation` (`self.Pick`))) (.y (`SceneComponent.RelativeLocation` (`self.Pick`))) (`KismetMathLibrary.FClamp` (select `bool` (`self.Up_Down_Direction`) :`false` (select `bool` (`local.Unlock_Status_Local`) :`false` (- _z 0.5) :`true` (- _z 0.75)) :`true` (+ _z 0.25)) (.z (`self.End_Pick_Location`)) (.z (`self.Start_Pick_Location`)))) true false)))))
      (else
        ;[1 1 1] Set pick start and end locations and do once
        (if (> (`self.Pick_Position`) 0)
          (set `self.Start_Pick_Location` _returnvalue_2)
          (else
            (set `self.Start_Pick_Location` _returnvalue_2)))
        (set `self.End_Pick_Location` (`KismetMathLibrary.MakeVector` (.x (`SceneComponent.RelativeLocation` (`self.Pick`))) (.y (`SceneComponent.RelativeLocation` (`self.Pick`))) (.z _end_location)))
        (set `self.Do_Once_Down` true)
        (set `local.Unlock_Status_Local` _random_result)
        (`self.Set_Section_Status` (`self.Pick_Position`) (`local.Unlock_Status_Local`))
        ;[1 1 1] Activate animations by status
        (bind _values (`BlueprintMapLibrary.Map_Values` (`self.Spawned_Sections`)))
        (if (`KismetArrayLibrary.Array_IsValidIndex` _values _returnvalue)
          (`self.Play_Stick_Down_Animation` (`|GetArrayItem` _values _returnvalue) (`local.Unlock_Status_Local`)))))
    (else
      ;[1 1 1] Remove this timer if movement timer are active
      (`KismetSystemLibrary.K2_ClearAndInvalidateTimerHandle` (`local.Timer Handle`)))))

(fn `Get Pick Down Location`
  (returns (`Random Result` :type Boolean) (`End Location` :type "Vector Structure"))
  (bind _can_activate (`self.Get_Random_By_Percents` (- (`self.Pick_Position`) 1)))
  (return _can_activate (`KismetMathLibrary.MakeVector` (.x (`SceneComponent.RelativeLocation` (`self.Pick`))) (.y (`SceneComponent.RelativeLocation` (`self.Pick`))) (select `bool` _can_activate :`false` 14.5 :`true` 14.0))))

(fn `Get Pick Location by Position`
  (params (`Pick Position` :type Integer))
  (returns (`End Location` :type "Vector Structure"))
  (bind _y (.y (`SceneComponent.RelativeLocation` (`self.Pick`))))
  (bind _z (.z (`SceneComponent.RelativeLocation` (`self.Pick`))))
  (bind _returnvalue (`KismetMathLibrary.MakeVector` -13.0 _y _z))
  (return (select `int` `Pick Position` :`0` _returnvalue :`1` _returnvalue :`2` (`KismetMathLibrary.MakeVector` -9.864 _y _z) :`3` (`KismetMathLibrary.MakeVector` -6.728 _y _z) :`4` (`KismetMathLibrary.MakeVector` -3.592 _y _z) :`5` (`KismetMathLibrary.MakeVector` -0.456 _y _z) :`6` (`KismetMathLibrary.MakeVector` 2.68 _y _z))))

(fn `Get_Random_By_Percents`
  (params (Stick_On_Work :type Integer))
  (returns (Can_Activate :type Boolean))
  (bind _sticks_enable_rand_percents (`self.Sticks_Enable_Rand_Percents`))
  (if (`KismetArrayLibrary.Array_IsValidIndex` _sticks_enable_rand_percents Stick_On_Work)
    (return (`KismetMathLibrary.InRange_IntInt` (`KismetMathLibrary.RandomIntegerInRange` 1 100) 1 (`|GetArrayItem` _sticks_enable_rand_percents Stick_On_Work)))
    (else
      (return false))))

(fn `Is Pick In Up Location`
  (returns (`Is Up Location` :type Boolean))
  (return (== (.z (`SceneComponent.RelativeLocation` (`self.Pick`))) 15.65)))

(fn `Move_Pick_Left`
  (params (Timer_Handle :type "TimerHandle Structure"))
  (bind _moving_to_right_timer (`self.Moving to Right Timer`))
  (if (`self.Is Pick In Up Location`)
    (if (`KismetSystemLibrary.K2_IsValidTimerHandle` _moving_to_right_timer)
      (`KismetSystemLibrary.K2_ClearAndInvalidateTimerHandle` _moving_to_right_timer))
    (if (`self.Do_Once_Left`)
      ;[1 1 1] Calculate is pick location on end location if not continue to change but if yes stop moving timer and reset do once.
      (if (== (`SceneComponent.RelativeLocation` (`self.Pick`)) (`self.End_Pick_Location`) :`ErrorTolerance` 0.1)
        (if (`KismetSystemLibrary.K2_IsTimerActiveHandle` (`local.Timer_Handle`))
          (`KismetSystemLibrary.K2_ClearAndInvalidateTimerHandle` (`local.Timer_Handle`))
          (set `self.Do_Once_Left` false))
        (else
          ;[1 1 1] Calculate how much need to move to right the Pick location and change it
          (`SceneComponent.K2_SetRelativeLocation` (`self.Pick`) (`KismetMathLibrary.MakeVector` (`KismetMathLibrary.FClamp` (- (.x (`SceneComponent.RelativeLocation` (`self.Pick`))) 0.5) (.x (`self.End_Pick_Location`)) (.x (`self.Start_Pick_Location`))) (.y (`SceneComponent.RelativeLocation` (`self.Pick`))) (.z (`SceneComponent.RelativeLocation` (`self.Pick`)))) false true)))
      (else
        ;[1 1 1] Set Start and End Locations of Pick
        (if (> (`self.Pick_Position`) 0)
          (set `self.Start_Pick_Location` (`self.Get Pick Location by Position` (+ (`self.Pick_Position`) 1)))
          (set `self.End_Pick_Location` (`self.Get Pick Location by Position` (`self.Pick_Position`)))
          (set `self.Do_Once_Left` true))))
    (else
      (`KismetSystemLibrary.K2_ClearAndInvalidateTimerHandle` (`local.Timer_Handle`)))))

(fn `Move_Pick_Right`
  (params (Timer_Handle :type "TimerHandle Structure"))
  (bind _moving_to_left_timer (`self.Moving to Left Timer`))
  (if (`self.Is Pick In Up Location`)
    (if (`KismetSystemLibrary.K2_IsTimerActiveHandle` (`self.Moving to Left Timer`))
      (`KismetSystemLibrary.K2_ClearAndInvalidateTimerHandle` _moving_to_left_timer :!label _label)
      (elif (`KismetSystemLibrary.K2_IsValidTimerHandle` _moving_to_left_timer)
        (goto _label)
        (else
          _)))
    (if (`self.Do_Once_Right`)
      ;[1 1 1] Calculate is pick location on end location if not continue to change but if yes stop moving timer and reset do once.
      (if (== (`SceneComponent.RelativeLocation` (`self.Pick`)) (`self.End_Pick_Location`) :`ErrorTolerance` 0.1)
        (if (`KismetSystemLibrary.K2_IsTimerActiveHandle` (`local.Timer_Handle`))
          (`KismetSystemLibrary.K2_ClearAndInvalidateTimerHandle` (`local.Timer_Handle`))
          (set `self.Do_Once_Right` false))
        (else
          ;[1 1 1] Calculate how much need to move to right the Pick location and change it
          (`SceneComponent.K2_SetRelativeLocation` (`self.Pick`) (`KismetMathLibrary.MakeVector` (`KismetMathLibrary.FClamp` (+ (.x (`SceneComponent.RelativeLocation` (`self.Pick`))) 0.5) (.x (`self.Start_Pick_Location`)) (.x (`self.End_Pick_Location`))) (.y (`SceneComponent.RelativeLocation` (`self.Pick`))) (.z (`SceneComponent.RelativeLocation` (`self.Pick`)))) false true)))
      (else
        ;[1 1 1] Set Start and End Locations of Pick
        (if (> (`self.Pick_Position`) 0)
          (set `self.Start_Pick_Location` (`self.Get Pick Location by Position` (- (`self.Pick_Position`) 1)))
          (else
            (set `self.Start_Pick_Location` (`self.Get Pick Location by Position` 1))))
        (set `self.End_Pick_Location` (`self.Get Pick Location by Position` (`self.Pick_Position`)))
        (set `self.Do_Once_Right` true)))
    (else
      (`KismetSystemLibrary.K2_ClearAndInvalidateTimerHandle` (`local.Timer_Handle`)))))

(fn `Play_Stick_Down_Animation`
  (params (Mesh :type "SkeletalMeshComponent Object Reference") (Unlock_Status :type Boolean))
  (`SkeletalMeshComponent.PlayAnimation` Mesh (select `bool` Unlock_Status :`false` "/Game/Advanced_Lock_Pick/Animations/Stick_SemiReturn_Animation.Stick_SemiReturn_Animation" :`true` "/Game/Advanced_Lock_Pick/Animations/Stick_FullDown_Animation.Stick_FullDown_Animation" :!type "AnimationAsset Object Reference") false))

(fn `Refresh Timers`
  (if (`KismetSystemLibrary.K2_IsValidTimerHandle` (`self.Moving to Right Timer`))
    (`KismetSystemLibrary.K2_ClearAndInvalidateTimerHandle` (`self.Moving to Right Timer`)))
  (if (`KismetSystemLibrary.K2_IsValidTimerHandle` (`self.Moving to Left Timer`))
    (`KismetSystemLibrary.K2_ClearAndInvalidateTimerHandle` (`self.Moving to Left Timer`))
    (return)
    (else
      (return))))

(fn `Return_All_Sticks_Def`
  (bind _spawned_sections (`self.Spawned_Sections`))
  (for _index (range (`BlueprintMapLibrary.Map_Length` (`self.Sections_Status`)))
    (bind _keys (`BlueprintMapLibrary.Map_Keys` _spawned_sections))
    (if (`KismetArrayLibrary.Array_IsValidIndex` _keys _index)
      (bind _values (`BlueprintMapLibrary.Map_Values` (`self.Sections_Status`)))
      (bind (_value _returnvalue) (`BlueprintMapLibrary.Map_Find` _spawned_sections (`|GetArrayItem` _keys _index)))
      (if _returnvalue
        (if (`|GetArrayItem` _values _index)
          (`SkeletalMeshComponent.PlayAnimation` _value "/Game/Advanced_Lock_Pick/Animations/Stick_FullReturn_Animation.Stick_FullReturn_Animation" false)))))
  (`self.Set_Section_Status` 0 false true))

(fn `Set_Section_Status`
  (params (`Section Index` :type Integer) (`Unlock Status` :type Boolean) (`Change all` :type Boolean :default false))
  (bind _sections_status (`self.Sections_Status`))
  (if `Change all`
    (`BlueprintMapLibrary.Map_Clear` _sections_status)
    (for _index (range (`KismetArrayLibrary.Array_Length` (`self.Sticks_Enumeration`)))
      (`BlueprintMapLibrary.Map_Add` (`self.Sections_Status`) (+ _index 1) `Unlock Status`))
    (else
      (bind _keys (`BlueprintMapLibrary.Map_Keys` _sections_status))
      (bind _values (`BlueprintMapLibrary.Map_Values` (`self.Sections_Status`)))
      (if (`KismetArrayLibrary.Array_IsValidIndex` _values (`KismetArrayLibrary.Array_Find` _keys `Section Index`))
        (bind _returnvalue (`BlueprintMapLibrary.Map_Remove` _sections_status `Section Index`))
        (if _returnvalue
          (`BlueprintMapLibrary.Map_Add` (`self.Sections_Status`) (`local.Section Index`) `Unlock Status`)
          ;[1 1 1] If all Sticks activated succesful call the Locker Unlocked Delegation
          (bind _values_2 (`BlueprintMapLibrary.Map_Values` (`self.Sections_Status`)))
          (if (not (`KismetArrayLibrary.Array_Contains` _values_2))
            (`self.On_Locker_Unlocked`)))))))

(fn `Stick Activation Conditions`
  (returns (`Can Continue to Next Stick` :type Boolean))
  (locals (`Finded Not Activated Previous` :type Boolean))
  (bind _returnvalue (- (`self.Pick_Position`) 1))
  (for _array_element (`self.Sticks_Enumeration`)
    (if (== _array_element (`self.Pick_Position`))
      (break)
      (else
        (bind (_value _returnvalue_2) (`BlueprintMapLibrary.Map_Find` (`self.Sections_Status`) _array_element))
        (if _returnvalue_2
          (if (not _value)
            (set `local.Finded Not Activated Previous` true)
            (return false))))))
  (if (`local.Finded Not Activated Previous`)
    ;[1 1 1] Play Fail Down Animation only to current Stick
    (bind _values (`BlueprintMapLibrary.Map_Values` (`self.Spawned_Sections`)))
    (if (`KismetArrayLibrary.Array_IsValidIndex` _values _returnvalue)
      (`self.Play_Stick_Down_Animation` (`|GetArrayItem` _values _returnvalue))
      (return false))
    (else
      (return true))))

(fn `Substract Pick_Position`
  (returns (`Is_Succes?` :type Boolean))
  (if (> (`self.Pick_Position`) 1)
    (if (`self.Is Pick In Up Location`)
      (bind _keys (`BlueprintMapLibrary.Map_Keys` (`self.Spawned_Sections`)))
      (set `self.Pick_Position` (`KismetMathLibrary.Clamp` (- (`self.Pick_Position`) 1) 1 (`KismetArrayLibrary.Array_Length` _keys)))
      (set `self.Do_Once_Left` false)
      (`self.Refresh Timers`)
      (`self.On_Pick_Moved_Left`)
      (return true)
      (else
        (return false)))
    (else
      (return false))))

(fn `UserConstructionScript`
  (`SceneCaptureComponent.ShowOnlyActorComponents` (`self.Render_Cam`) self true))